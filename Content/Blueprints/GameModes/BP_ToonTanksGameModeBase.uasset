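; Game mode Blueprint for Toon Tanks that drives the player HUD through the game's countdown, gameplay and game-over phases.
; BeginPlay creates and caches the WBP_Player widget, which the other events update with countdown, turret count and health ratio.
; GameOver passes the win/loss result to the widget, then reloads the current level after a short delay.
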(event `self.ReceiveBeginPlay`
  (bind _returnvalue (`|CreateWidget` (`self.WidgetClass`)))
  (bind _aswbp_player (cast `/Game/Blueprints/Widgets/WBP_Player` _returnvalue))
  (bind _output_get (set `self.As WBP Player` _aswbp_player))
  (`UserWidget.AddToViewport` _output_get 0))

(event `self.StartCountdown`
  (bind _as_wbp_player (`self.As WBP Player`))
  (`/Engine/EditorBlueprintResources/StandardMacros.IsValid` _as_wbp_player
    (:`Is Valid`
      (bind _result (`/Engine/EditorBlueprintResources/StandardMacros.IncrementInt` (`self.StartDelay_`))
        (:`  `
          (`/Game/Blueprints/Widgets/WBP_Player.SetCountdownTimer` _as_wbp_player (`KismetMathLibrary.Conv_IntToDouble` _result)))))))

(event `self.StartGameplay`
  (bind _as_wbp_player (`self.As WBP Player`))
  (`/Engine/EditorBlueprintResources/StandardMacros.IsValid` _as_wbp_player
    (:`Is Valid`
      (`/Game/Blueprints/Widgets/WBP_Player.StateStart_Gameplay` _as_wbp_player)
      (`/Game/Blueprints/Widgets/WBP_Player.StateFinish_Countdown` _as_wbp_player)
      (`/Game/Blueprints/Widgets/WBP_Player.UpdateEnemyCount` _as_wbp_player (`self.TargetTurretCount_`))
      (`/Game/Blueprints/Widgets/WBP_Player.UpdateHealthBar` _as_wbp_player 1.0))))

(event `self.GameOver`
  (params (bHasWon :type Boolean))
  (bind _as_wbp_player (`self.As WBP Player`))
  (`/Engine/EditorBlueprintResources/StandardMacros.IsValid` _as_wbp_player
    (:`Is Valid`
      (`/Game/Blueprints/Widgets/WBP_Player.SetHasWon` _as_wbp_player bHasWon)
      (`KismetSystemLibrary.Delay` 3.0)
      (bind _returnvalue (`GameplayStatics.GetCurrentLevelName` true))
      (`GameplayStatics.OpenLevel` (`KismetStringLibrary.Conv_StringToName` _returnvalue)))))

(event `self.TurretDead`
  (params (TurretCount :type Integer))
  (bind _as_wbp_player (`self.As WBP Player`))
  (`/Engine/EditorBlueprintResources/StandardMacros.IsValid` _as_wbp_player
    (:`Is Valid`
      (`/Game/Blueprints/Widgets/WBP_Player.UpdateEnemyCount` _as_wbp_player TurretCount))))

(event `self.PlayerDamaged`
  (params (HealthRatio :type "Float (single-precision)"))
  (bind _as_wbp_player (`self.As WBP Player`))
  (`/Engine/EditorBlueprintResources/StandardMacros.IsValid` _as_wbp_player
    (:`Is Valid`
      (`/Game/Blueprints/Widgets/WBP_Player.UpdateHealthBar` _as_wbp_player HealthRatio))))

(fn `UserConstructionScript`)